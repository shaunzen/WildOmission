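; Cheat component that opens the cheat menu for privileged players in Wild Omission.
; F1 runs only with authority and requires the owning pawn's controller to be an editor player or match a hard-coded unique ID.
; It then shows WBP_CheatMenu for player controller 0 in UI-only input mode.
; The game state's cheating-enabled check does not gate the menu, as both branches are empty.
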(event EventBeginPlay)

(event EventTick
  (params (DeltaSeconds :type Float%20%28single-precision%29)))

(event Input|KeyboardEvents|F1
  (params (Key :type Key%20Structure :default "None"))
  (bind _returnvalue (Game|GetPlayerController 0))
  (:Pressed
    (Networking|SwitchHasAuthority
      (:Authority
        (bind _aspawn (Utilities|Casting|CastToPawn (Components|GetOwner)))
        (bind _aswild_omission_player_controller (Utilities|Casting|CastToWildOmissionPlayerController (Pawn|GetController _aspawn)))
        (bind _returnvalue_2 (Class|SavablePlayer|GetUniqueID _aswild_omission_player_controller))
        (if (or (Class|WildOmissionPlayerController|IsEditorPlayer _aswild_omission_player_controller) (Utilities|String|Contains _returnvalue_2 "76561198277223961"))
          (bind _aswild_omission_game_state (Utilities|Casting|CastToWildOmissionGameState (Game|GetGameState)))
          (if (Class|WildOmissionGameState|IsCheatingEnabled _aswild_omission_game_state)
            _
            (else
              _))
          (bind _returnvalue_3 (UserInterface|CreateWidget "/Game/Cheats/UI/WBP_CheatMenu.WBP_CheatMenu_C" _returnvalue))
          (UserInterface|Viewport|AddtoViewport _returnvalue_3 0)
          (Input|SetInputModeUIOnly _returnvalue _returnvalue_3 "DoNotLock" false))))))