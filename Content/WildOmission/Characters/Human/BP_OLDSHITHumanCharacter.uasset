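; Legacy human character Blueprint, marked old by its name, that adds Escape-key menu handling.
; Escape checks the HUD widget for an open menu, closing it if one exists or otherwise showing the gameplay menu through the WildOmission game instance.
; Closing toggles the inventory menu if open, then crafting, and otherwise falls back to toggling chat.
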(event EventBeginPlay)

(event Collision|EventActorBeginOverlap
  (params (OtherActor :type Actor%20Object%20Reference)))

(event EventTick
  (params (DeltaSeconds :type Float%20%28single-precision%29)))

(event Input|KeyboardEvents|Escape
  (params (Key :type Key%20Structure))
  ;[1 1 1] Show Gameplay Menu
  (:Pressed
    (if (Class|PlayerHUDWidget|IsMenuOpen (Class|WildOmissionCharacter|GetHUDWidget))
      (CallFunction|CloseMenu)
      (else
        (CallFunction|ShowGameplayMenu)))))

(fn ConstructionScript)

(fn ShowGameplayMenu
  (bind _aswild_omission_game_instance (Utilities|Casting|CastToWildOmissionGameInstance (Game|GetGameInstance)))
  (Class|WildOmissionGameInstance|ShowGameplayMenuWidget _aswild_omission_game_instance))

(fn CloseMenu
  (bind _returnvalue (Class|WildOmissionCharacter|GetHUDWidget))
  (if (Class|PlayerHUDWidget|IsInventoryMenuOpen _returnvalue)
    (Class|PlayerHUDWidget|ToggleInventoryMenu _returnvalue)
    (elif (Class|PlayerHUDWidget|IsCraftingMenuOpen _returnvalue)
      (Class|PlayerHUDWidget|ToggleCraftingMenu _returnvalue)
      (else
        (Class|PlayerHUDWidget|ToggleChatMenu _returnvalue)))))